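; Rocket launcher actor that fires BP_Rocket projectiles from a limited Bullets count.
; It enables player 0 input on BeginPlay and handles the Fire action itself.
; Each shot spawns a rocket at the mesh location plus a camera-rotated offset, plays two sounds there, and decrements Bullets.
; Aim comes from the player camera manager's rotation, avoiding hard references to the character.
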(event `InputAction|Fire`
  (params (Key :type "Key Structure"))
  (bind _returnvalue (`PlayerCameraManager.GetCameraRotation` (`GameplayStatics.GetPlayerCameraManager` 0)))
  (bind _returnvalue_2 (+ (`SceneComponent.K2_GetComponentLocation` (`self.StaticMesh`)) (`KismetMathLibrary.GreaterGreater_VectorRotator` (`self.Projectile Offset`) _returnvalue)))
  (:`Pressed`
    (if (> (`self.Bullets`) 0)
      (`|SpawnActorFromClass` "/Game/FirstPerson/Blueprints/BP_Rocket.BP_Rocket_C" (`KismetMathLibrary.MakeTransform` _returnvalue_2 _returnvalue) "Undefined" "OverrideRootScale" null null)
      (`GameplayStatics.PlaySoundAtLocation` "/Game/Audio/Rocket.Rocket" _returnvalue_2 (struct) 1.0 1.0 0.0 null null null null) ; Play firing sound
      (`GameplayStatics.PlaySoundAtLocation` "/Game/FPWeapon/Audio/FirstPersonTemplateWeaponFire02.FirstPersonTemplateWeaponFire02" _returnvalue_2 (struct) 1.0 1.0 0.0 null null null null) ; Play firing sound
      (`/Engine/EditorBlueprintResources/StandardMacros.DecrementInt` (`self.Bullets`)))))

(event `self.ReceiveBeginPlay`
  (`self.EnableInput` (`GameplayStatics.GetPlayerController` 0)))

(fn `UserConstructionScript`)