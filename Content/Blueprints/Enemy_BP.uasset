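; Enemy actor that wanders the navmesh while facing and shooting at the first-person player, and can be killed.
; A self-repeating Roam loop moves it to random reachable points with random pauses, whether each move succeeds or fails.
; Tick turns its capsule toward the player, and a Delay throttles Shoot, a debug-drawn forward trace with slight random offset that calls HealDamage on the player.
; TakeDamage lowers Health, printing a win message and destroying it at zero.
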(event `Roam`
  ; Roam
  (bind _randomlocation (`NavigationSystemV1.K2_GetRandomLocationInNavigableRadius` (`SceneComponent.K2_GetComponentLocation` (`self.Mesh`)) 10000.0 null null))
  (`|AIMoveTo` self _randomlocation null
    (:`OnSuccess`
      _)
    (:`OnFail`
      _))
  (`KismetSystemLibrary.Delay` (`KismetMathLibrary.RandomFloatInRange` 0.1 3.0))
  (`self.Roam`))

(event `Shoot`
  (bind _capsulecomponent (`self.CapsuleComponent`))
  (bind _returnvalue (`SceneComponent.K2_GetComponentLocation` _capsulecomponent))
  ; Shoot
  (bind _outhit (`KismetSystemLibrary.LineTraceSingle` :`Start` _returnvalue :`End` (+ (+ _returnvalue (* (`SceneComponent.GetForwardVector` _capsulecomponent) 10000.0)) (`KismetMathLibrary.MakeVector` (`KismetMathLibrary.RandomFloatInRange` 0.0 10.0) (`KismetMathLibrary.RandomFloatInRange` 0.0 10.0) (`KismetMathLibrary.RandomFloatInRange` 0.0 10.0))) :`TraceChannel` "TraceTypeQuery2" :`DrawDebugType` "ForDuration"))
  (bind _asbp_first_person_character (cast `/Game/FirstPerson/Blueprints/BP_FirstPersonCharacter` (`.HitActor` (`GameplayStatics.BreakHitResult` _outhit))))
  (`/Game/FirstPerson/Blueprints/BP_FirstPersonCharacter.Heal/Damage` _asbp_first_person_character (`self.Damage`)))

(event `self.ReceiveBeginPlay`
  ; Begin Play
  (`self.Roam`)
  (bind _asbp_first_person_character (cast `/Game/FirstPerson/Blueprints/BP_FirstPersonCharacter` (`GameplayStatics.GetPlayerCharacter` 0)))
  (set `self.FP_BP` _asbp_first_person_character))

(event `self.ReceiveTick`
  (params (DeltaSeconds :type "Float (single-precision)"))
  ; Look At
  (`|ExecutionSequence`
    (:`then_0`
      (`SceneComponent.K2_SetWorldRotation` (`self.CapsuleComponent`) (`KismetMathLibrary.FindLookAtRotation` (`SceneComponent.K2_GetComponentLocation` (`self.CapsuleComponent`)) (`SceneComponent.K2_GetComponentLocation` (`Actor.RootComponent` (`self.FP_BP`)))) false false))
    (:`then_1`
      (`KismetSystemLibrary.Delay` 0.5)
      (`self.Shoot`))))

(event `TakeDamage`
  (params (Value :type "Float (double-precision)"))
  ; Take Damage
  (bind _output_get (set `self.Health` (- (`self.Health`) Value)))
  (`KismetSystemLibrary.PrintString` (`KismetStringLibrary.Conv_DoubleToString` _output_get))
  (if (<= _output_get 0.0)
    (`KismetSystemLibrary.PrintString` "You Win")
    (`self.K2_DestroyActor`)))

(fn `UserConstructionScript`)