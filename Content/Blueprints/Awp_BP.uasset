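; Awp_BP is a sniper rifle actor with a toggled scope and hitscan firing.
; Zoom flips the scope overlay on UNO_BP's HUD, hides the rifle and narrows the first-person camera FOV, then restores them.
; Fire, while bullets remain, plays a shot sound, line-traces from the camera with debug drawing, spends a bullet and damages any Enemy_BP hit.
; BeginPlay enables input and caches the character and UNO_BP references.
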(event `InputAction|Zoom`
  (params (Key :type "Key Structure"))
  (bind _hud (`/Game/Blueprints/UNO_BP.HUD` (`self.UNO_BP`)))
  (bind _firstpersoncamera (`/Game/FirstPerson/Blueprints/BP_FirstPersonCharacter.FirstPersonCamera` (`self.FP_BP`)))
  ; Shoot
  (:`Pressed`
    (`/Engine/EditorBlueprintResources/StandardMacros.FlipFlop`
      (:`A`
        (set `/Game/WBP/HUD_WBP.ScopeVis` "Visible" _hud)
        (`self.SetActorHiddenInGame` true)
        (`CameraComponent.SetFieldOfView` _firstpersoncamera 60.0))
      (:`B`
        (set `/Game/WBP/HUD_WBP.ScopeVis` "Hidden" _hud)
        (`self.SetActorHiddenInGame` false)
        (`CameraComponent.SetFieldOfView` _firstpersoncamera 90.0)))))

(event `InputAction|Fire`
  (params (Key :type "Key Structure"))
  (bind _firstpersoncamera (`/Game/FirstPerson/Blueprints/BP_FirstPersonCharacter.FirstPersonCamera` (`self.FP_BP`)))
  (bind _returnvalue (`SceneComponent.K2_GetComponentLocation` _firstpersoncamera))
  ; Shoot
  (:`Pressed`
    (set `self.Shooting` true)
    (if (> (`self.Bullets`) 0)
      (`GameplayStatics.PlaySound2D` "/Game/Audio/Sniper.Sniper" 1.0 1.0 0.0 null null)
      (bind _outhit (`KismetSystemLibrary.LineTraceSingle` :`Start` _returnvalue :`End` (+ _returnvalue (* (`self.Distance`) (`SceneComponent.GetForwardVector` _firstpersoncamera))) :`TraceChannel` "TraceTypeQuery1" :`DrawDebugType` "ForDuration"))
      (`/Engine/EditorBlueprintResources/StandardMacros.DecrementInt` (`self.Bullets`)
        (:`  `
          (bind _asenemy_bp (cast `/Game/Blueprints/Enemy_BP` (`.HitActor` (`GameplayStatics.BreakHitResult` _outhit))))
          (`/Game/Blueprints/Enemy_BP.TakeDamage` _asenemy_bp (`self.Damage`))))))
  (:`Released`
    (set `self.Shooting` false)))

(event `self.ReceiveBeginPlay`
  (`self.EnableInput` (`GameplayStatics.GetPlayerController` 0))
  (bind _asbp_first_person_character (cast `/Game/FirstPerson/Blueprints/BP_FirstPersonCharacter` (`GameplayStatics.GetPlayerCharacter` 0)))
  (set `self.FP_BP` _asbp_first_person_character)
  (bind _returnvalue (`GameplayStatics.GetActorOfClass` "/Game/Blueprints/UNO_BP.UNO_BP_C"))
  (set `self.UNO_BP` _returnvalue))

(fn `UserConstructionScript`)