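; UNO_BP manages the player's UNO-style card hand, where playing a card updates the first-person character's gun.
; BeginPlay creates the HUD widget, enables input and deals a random starting hand from PossibleCards.
; Number keys play the card in the matching slot: it becomes ActiveCard, leaves the hand and triggers SetGun on the character.
; DrawCard adds a random card unless the hand holds ten, and hand changes re-render the HUD.
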(event `Key|One`
  (params (Key :type "Key Structure"))
  ; Hot Keys
  (:`Pressed`
    (`self.PlayCard` (`|GetArrayItem` (`self.PlayerCards`)))))

(event `Key|Six`
  (params (Key :type "Key Structure"))
  ; Hot Keys
  (:`Pressed`
    (`self.PlayCard` (`|GetArrayItem` (`self.PlayerCards`) 5) 5)))

(event `Key|Two`
  (params (Key :type "Key Structure"))
  ; Hot Keys
  (:`Pressed`
    (`self.PlayCard` (`|GetArrayItem` (`self.PlayerCards`) 1) 1)))

(event `Key|Seven`
  (params (Key :type "Key Structure"))
  ; Hot Keys
  (:`Pressed`
    (`self.PlayCard` (`|GetArrayItem` (`self.PlayerCards`) 6) 6)))

(event `Key|Eight`
  (params (Key :type "Key Structure"))
  ; Hot Keys
  (:`Pressed`
    (`self.PlayCard` (`|GetArrayItem` (`self.PlayerCards`) 7) 7)))

(event `Key|Three`
  (params (Key :type "Key Structure"))
  ; Hot Keys
  (:`Pressed`
    (`self.PlayCard` (`|GetArrayItem` (`self.PlayerCards`) 2) 2)))

(event `Key|Nine`
  (params (Key :type "Key Structure"))
  ; Hot Keys
  (:`Pressed`
    (`self.PlayCard` (`|GetArrayItem` (`self.PlayerCards`) 8) 8)))

(event `Key|Four`
  (params (Key :type "Key Structure"))
  ; Hot Keys
  (:`Pressed`
    (`self.PlayCard` (`|GetArrayItem` (`self.PlayerCards`) 3) 3)))

(event `Key|Zero`
  (params (Key :type "Key Structure"))
  ; Hot Keys
  (:`Pressed`
    (`self.PlayCard` (`|GetArrayItem` (`self.PlayerCards`) 9) 9)))

(event `Key|Five`
  (params (Key :type "Key Structure"))
  ; Hot Keys
  (:`Pressed`
    (`self.PlayCard` (`|GetArrayItem` (`self.PlayerCards`) 4) 4)))

(event `self.ReceiveBeginPlay`
  ; Begin Play
  (bind _returnvalue (`|CreateWidget` "/Game/WBP/HUD_WBP.HUD_WBP_C" (`GameplayStatics.GetPlayerController` 0)))
  (bind _output_get (set `self.HUD` _returnvalue))
  (`UserWidget.AddToViewport` _output_get 0)
  (`self.Create Starting Deck`)
  (`self.EnableInput` (`GameplayStatics.GetPlayerController` 0)))

(event `PlayCard`
  (params (ActiveCard :type "/Game/Blueprints/Card Structure") (IndexToRemove :type Integer))
  ; Play Card
  (set `self.ActiveCard` ActiveCard)
  (`KismetArrayLibrary.Array_Remove` (`self.PlayerCards`) IndexToRemove)
  (`self.ReRender`)
  (bind _asbp_first_person_character (cast `/Game/FirstPerson/Blueprints/BP_FirstPersonCharacter` (`GameplayStatics.GetPlayerCharacter` 0)))
  (`/Game/FirstPerson/Blueprints/BP_FirstPersonCharacter.SetGun` _asbp_first_person_character))

(event `DrawCard`
  ; Draw Card
  (if (not (== (`KismetArrayLibrary.Array_Length` (`self.PlayerCards`)) 10))
    (bind _card (`self.RandomCard`))
    (`KismetArrayLibrary.Array_Add` (`self.PlayerCards`) _card)
    (`self.ReRender`)))

(event `ReRender`
  ; Render
  (`/Game/WBP/HUD_WBP.RenderCards` (`self.HUD`)))

(event `Create Starting Deck`
  ; Create Starting Deck
  (for _ (range (+ (`self.StartingDeckSize`) 1))
    (bind _card (`self.RandomCard`))
    (`KismetArrayLibrary.Array_Add` (`self.PlayerCards`) _card)
    (`self.ReRender`)))

(fn `RandomCard`
  (returns (Card :type "/Game/Blueprints/Card Structure"))
  (bind _possiblecards (`self.PossibleCards`))
  (return (`|GetArrayItem` _possiblecards (`KismetMathLibrary.RandomInteger` (`KismetArrayLibrary.Array_Length` _possiblecards)))))

(fn `UserConstructionScript`)