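; MiniGun_BP is an automatic weapon actor that takes the player's Fire input and references the first-person character on BeginPlay.
; Holding Fire starts a looping timer that fires rapid hitscan line traces from the character's camera.
; Each shot uses a bullet, shows the muzzle flash, plays a sound and damages any Enemy_BP hit.
; Releasing Fire or running out of bullets clears the timer and hides the flash.
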(event `Shoot`
  (bind _ns_muzzleflash (`self.NS_MuzzleFlash`))
  (bind _firstpersoncamera (`/Game/FirstPerson/Blueprints/BP_FirstPersonCharacter.FirstPersonCamera` (`self.FP_BP`)))
  (bind _returnvalue (`SceneComponent.K2_GetComponentLocation` _firstpersoncamera))
  ; Shoot
  (if (> (`self.Bullets`) 0)
    (bind _outhit (`KismetSystemLibrary.LineTraceSingle` :`Start` _returnvalue :`End` (+ _returnvalue (* (`self.Distance`) (`SceneComponent.GetForwardVector` _firstpersoncamera))) :`TraceChannel` "TraceTypeQuery1" :`DrawDebugType` "ForDuration"))
    (`/Engine/EditorBlueprintResources/StandardMacros.DecrementInt` (`self.Bullets`)
      (:`  `
        (`SceneComponent.SetVisibility` _ns_muzzleflash true false)
        (`GameplayStatics.PlaySound2D` "/Game/Audio/UZI.UZI" 1.0 1.0 0.0 null null)
        (bind _asenemy_bp (cast `/Game/Blueprints/Enemy_BP` (`.HitActor` (`GameplayStatics.BreakHitResult` _outhit))))
        (`/Game/Blueprints/Enemy_BP.TakeDamage` _asenemy_bp (`self.Damage`))))
    (else
      (`SceneComponent.SetVisibility` _ns_muzzleflash false false :!label _label)
      (`KismetSystemLibrary.K2_ClearAndInvalidateTimerHandle` (stale `InputAction|Fire` _output_get)))))

(event `InputAction|Fire`
  (params (Key :type "Key Structure"))
  ; Shoot
  (:`Pressed`
    (set `self.Shooting` true)
    (bind _returnvalue (`KismetSystemLibrary.K2_SetTimerDelegate` (delegate `Shoot`) 0.05 true))
    (bind _output_get (set `self.Timer` _returnvalue)))
  (:`Released`
    (set `self.Shooting` false)
    (goto _label)))

(event `self.ReceiveBeginPlay`
  (`self.EnableInput` (`GameplayStatics.GetPlayerController` 0))
  (bind _asbp_first_person_character (cast `/Game/FirstPerson/Blueprints/BP_FirstPersonCharacter` (`GameplayStatics.GetPlayerCharacter` 0)))
  (set `self.FP_BP` _asbp_first_person_character))

(fn `UserConstructionScript`)